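; Actor component that moves its owner along an array of waypoints in Once, Back and Forth or Loop mode.
; On BeginPlay it places the owner at the first waypoint, then a looping timer, rather than Tick, applies constant steps sized to each leg's travel time.
; On arrival it optionally pauses, snaps to the waypoint and selects the next.
; Waypoints can override default travel and wait times.
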(event Custom|Step
  (bind _owner (Variables|Default|GetOwner))
  (Transformation|SetActorLocation _owner (+ (Transformation|GetActorLocation _owner) (Variables|Default|GetCurrentStep)) true false)
  (if (Utilities|Operators|EqualEqual (Transformation|GetActorLocation (Variables|Default|GetOwner)) (Transformation|GetActorLocation (CallFunction|GetNextWaypoint)) 0.01)
    (if (> (Variables|Default|GetCurrentTimeOnWaypoint) 0.0)
      (Utilities|Time|PauseTimerbyHandle (Variables|Default|GetTimerHandle))
      (Utilities|Time|SetTimerbyEvent (delegate Custom|WaitOnWaypoint) (Variables|Default|GetCurrentTimeOnWaypoint))
      (else
        (Transformation|SetActorLocation (Variables|Default|GetOwner) (Transformation|GetActorLocation (CallFunction|GetNextWaypoint)) false false)
        (CallFunction|WaypointReached)
        (Utilities|Time|UnpauseTimerbyHandle (Variables|Default|GetTimerHandle))))))

(event Custom|StartMoving
  (if (Math|Integer|InRange(Integer) (Variables|Default|GetNextWaypoint) 0 (Utilities|Array|Length (Variables|Setup|GetWaypoints)) true false)
    (bind _returnvalue (Utilities|Time|SetTimerbyEvent (delegate Custom|Step) (Variables|Setup|GetStepTime) true))
    (Variables|Default|SetTimerHandle _returnvalue)))

(event Custom|WaypointReached
  (bind _nextwaypoint (CallFunction|FindNextWaypointIndex))
  (Variables|Default|SetNextWaypoint _nextwaypoint)
  (if (Math|Integer|InRange(Integer) (Variables|Default|GetNextWaypoint) 0 (Utilities|Array|Length (Variables|Setup|GetWaypoints)) true false)
    (CallFunction|UpdateMovementValues (CallFunction|GetNextWaypoint))
    (else
      (CallFunction|StopMoving))))

(event Custom|WaitOnWaypoint
  (Transformation|SetActorLocation (Variables|Default|GetOwner) (Transformation|GetActorLocation (CallFunction|GetNextWaypoint)) false false)
  (CallFunction|WaypointReached)
  (Utilities|Time|UnpauseTimerbyHandle (Variables|Default|GetTimerHandle)))

(event Custom|StopMoving
  (Utilities|Time|ClearandInvalidateTimerbyHandle (Variables|Default|GetTimerHandle)))

(event EventBeginPlay
  (if (Utilities|Array|IsValidIndex (Variables|Setup|GetWaypoints))
    (bind _output_get (Variables|Default|SetOwner (Components|GetOwner)))
    (Transformation|SetActorLocation _output_get (Transformation|GetActorLocation (Utilities|Array|Get(acopy) (Variables|Setup|GetWaypoints))) true false)
    (CallFunction|UpdateMovementValues (CallFunction|GetNextWaypoint))
    (CallFunction|StartMoving)))

(fn UpdateMovementValues
  (params (NextWaypoint :type BP%20Xe%20Waypoint%20Object%20Reference))
  (bind _returnvalue (Transformation|GetActorLocation NextWaypoint))
  (bind _owner (Variables|Default|GetOwner))
  (bind _returnvalue_2 (Transformation|GetActorLocation _owner))
  (bind _returnvalue_3 (- _returnvalue _returnvalue_2))
  (Utilities|IsValid NextWaypoint
    (:Is%20Valid
      (Variables|Default|SetCurrentTimeToReach (Math|Float|SelectFloat (Variables|/XeProtoWaypointMovement/XeProtoWaypointMovement/Blueprint/BP_XeWaypoint.BP_XeWaypoint_C|GetCustomTimeToReach NextWaypoint) (Variables|DefaultValues|GetDefaultTimeToReach) (Variables|/XeProtoWaypointMovement/XeProtoWaypointMovement/Blueprint/BP_XeWaypoint.BP_XeWaypoint_C|GetOverrideTimeToReach NextWaypoint)))
      (Variables|Default|SetCurrentTimeOnWaypoint (Math|Float|SelectFloat (Variables|/XeProtoWaypointMovement/XeProtoWaypointMovement/Blueprint/BP_XeWaypoint.BP_XeWaypoint_C|GetCustomTimeOnWaypoint NextWaypoint) (Variables|DefaultValues|GetDefaultTimeOnWaipoint) (Variables|/XeProtoWaypointMovement/XeProtoWaypointMovement/Blueprint/BP_XeWaypoint.BP_XeWaypoint_C|GetOverrideTimeOnWaypoint NextWaypoint)))
      (Variables|Default|SetCurrentStep (* (Math|Vector|Normalize _returnvalue_3) (* (/ (Math|Vector|VectorLength _returnvalue_3) (Variables|Default|GetCurrentTimeToReach)) (Variables|Setup|GetStepTime)))))))

(fn GetNextWaypoint
  (return (Utilities|Array|Get(acopy) (Variables|Setup|GetWaypoints) (Variables|Default|GetNextWaypoint))))

(fn FindNextWaypointIndex
  (switch Utilities|FlowControl|Switch|SwitchonE_XeWaypointMovementType (Variables|Setup|GetMovementType)
    (:NewEnumerator0
      (if (== (Variables|Default|GetNextWaypoint) (- (Utilities|Array|Length (Variables|Setup|GetWaypoints)) 1))
        (Variables|Default|SetNextWaypoint -1)
        (else
          (Variables|Default|SetNextWaypoint (+ (Variables|Default|GetNextWaypoint) (Variables|Default|GetNextWaypointDirection)) :!label _label))))
    (:NewEnumerator1
      (if (not (Math|Integer|InRange(Integer) (Variables|Default|GetNextWaypoint) 0 (- (Utilities|Array|Length (Variables|Setup|GetWaypoints)) 1) false false))
        (Variables|Default|SetNextWaypointDirection (* (Variables|Default|GetNextWaypointDirection) -1))
        (goto _label)
        (else
          (goto _label))))
    (:NewEnumerator2
      (if (== (Variables|Default|GetNextWaypoint) (- (Utilities|Array|Length (Variables|Setup|GetWaypoints)) 1))
        (Variables|Default|SetNextWaypoint 0)
        (else
          (goto _label)))))
  (return (Variables|Default|GetNextWaypoint)))